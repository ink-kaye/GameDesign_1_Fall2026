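; Interactive seven-part sculpture, used as a child actor of BP_Infinity_Sculpture, whose UI it opens when clicked.
; TriggerInteraction lerps each mesh between original transforms cached at BeginPlay and target transforms, playing delayed forward or backward sounds.
; Separate events toggle a lift-and-tilt levitation and decor visibility.
; BeginPlay also collects MI_Emissive_ materials as dynamic instances, letting functions toggle glow by parameter or material swap.
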(event `self.ReceiveBeginPlay`
  (bind _array (`|MakeArray` (`self.Mesh_03`) (`self.Mesh_04`) (`self.Mesh_06`) (`self.Mesh_07`) (`self.Mesh_05`) (`self.Mesh_02`) (`self.Mesh_01`)))
  (`|ExecutionSequence`
    (:`then_0`
      ;[0 0 0] Array
      (set `self.MeshComponentsArray` _array)
      (set `self.MeshesToCheck` _array)
      (`KismetArrayLibrary.Array_Clear` (`self.OriginalMaterialsArray`))
      (`KismetArrayLibrary.Array_Clear` (`self.EmissiveMIDs`))
      (`KismetArrayLibrary.Array_Clear` (`self.EmissiveDefaultStrengths`))
      (for _array_element (`self.MeshesToCheck`)
        (for _index (range (`PrimitiveComponent.GetNumMaterials` _array_element))
          (bind _returnvalue (`PrimitiveComponent.GetMaterial` _array_element _index))
          (if (`KismetStringLibrary.StartsWith` (`KismetSystemLibrary.GetObjectName` _returnvalue) "MI_Emissive_")
            (bind _returnvalue_2 (`PrimitiveComponent.CreateDynamicMaterialInstance` _array_element _index _returnvalue "None"))
            (bind _returnvalue_3 (`MaterialInstanceDynamic.K2_GetScalarParameterValue` _returnvalue_2 "EmissiveStrength"))
            (`KismetArrayLibrary.Array_Add` (`self.EmissiveMIDs`) _returnvalue_2)
            (`KismetArrayLibrary.Array_Add` (`self.EmissiveDefaultStrengths`) _returnvalue_3)
            (`KismetArrayLibrary.Array_Add` (`self.EmissiveMeshComponents`) _array_element)
            (`KismetArrayLibrary.Array_Add` (`self.EmissiveMaterialIndices`) _index)
            (`KismetArrayLibrary.Array_Add` (`self.OriginalEmissiveMaterials`) _returnvalue)))))
    (:`then_1`
      (`self.OriginalLocation`))))

(event `self.ReceiveActorOnClicked`
  (params (ButtonPressed :type "Key Structure"))
  ;[0 0 0] Comment
  (bind _asbp_infinity_sculpture (cast `/Game/InfinityAssets/BP/Sculpture/BP_Infinity_Sculpture` (`self.GetParentActor`)))
  (`/Game/InfinityAssets/BP/Sculpture/BP_Infinity_Sculpture.ForceOpenUI` _asbp_infinity_sculpture))

(event `/Game/InfinityAssets/BP/Sculpture/BPI_InfinityTrigger.TriggerInteraction`
  (`/Engine/EditorBlueprintResources/StandardMacros.FlipFlop`
    (:`A`
      (`|ExecutionSequence`
        (:`then_0`
          (`KismetSystemLibrary.Delay` 1.0)
          ;[0 0 0] Animation
          (if (`self.TriggerInteraction?`)
            (set `self.TriggerInteraction?` false)
            (`|ExecutionSequence`
              (:`then_0`
                (bind (_direction _alpha) (`Timeline|AnimationTimeline` :!label _label)
                  (:`Update`
                    (set `self.Alpha` _alpha)
                    (`SceneComponent.K2_SetRelativeRotation` (`self.Mesh_01`) (`KismetMathLibrary.RLerp` (`self.OriginalRotation_1`) (`self.Mesh_1_Rotation`) (`self.Alpha`)) false false)
                    (`SceneComponent.K2_SetRelativeLocation` (`self.Mesh_01`) (`KismetMathLibrary.VLerp` (`self.OriginalLocation_1`) (`self.Mesh_1_Location`) (`self.Alpha`)) false false)
                    (`SceneComponent.SetRelativeScale3D` (`self.Mesh_01`) (`KismetMathLibrary.VLerp` (`self.Original Scale 1`) (`self.Mesh_1_Scale`) (`self.Alpha`)))
                    (`SceneComponent.K2_SetRelativeRotation` (`self.Mesh_02`) (`KismetMathLibrary.RLerp` (`self.OriginalRotation_2`) (`self.Mesh_2_Rotation`) (`self.Alpha`)) false false)
                    (`SceneComponent.K2_SetRelativeLocation` (`self.Mesh_02`) (`KismetMathLibrary.VLerp` (`self.OriginalLocation_2`) (`self.Mesh_2_Location`) (`self.Alpha`)) false false)
                    (`SceneComponent.SetRelativeScale3D` (`self.Mesh_02`) (`KismetMathLibrary.VLerp` (`self.Original Scale 2`) (`self.Mesh_2_Scale`) (`self.Alpha`)))
                    (`SceneComponent.K2_SetRelativeRotation` (`self.Mesh_03`) (`KismetMathLibrary.RLerp` (`self.OriginalRotation_3`) (`self.Mesh_3_Rotation`) (`self.Alpha`)) false false)
                    (`SceneComponent.K2_SetRelativeLocation` (`self.Mesh_03`) (`KismetMathLibrary.VLerp` (`self.OriginalLocation_3`) (`self.Mesh_3_Location`) (`self.Alpha`)) false false)
                    (`SceneComponent.SetRelativeScale3D` (`self.Mesh_03`) (`KismetMathLibrary.VLerp` (`self.Original Scale 3`) (`self.Mesh_3_Scale`) (`self.Alpha`)))
                    (`SceneComponent.K2_SetRelativeRotation` (`self.Mesh_04`) (`KismetMathLibrary.RLerp` (`self.OriginalRotation_4`) (`self.Mesh_4_Rotation`) (`self.Alpha`)) false false)
                    (`SceneComponent.K2_SetRelativeLocation` (`self.Mesh_04`) (`KismetMathLibrary.VLerp` (`self.OriginalLocation_4`) (`self.Mesh_4_Location`) (`self.Alpha`)) false false)
                    (`SceneComponent.SetRelativeScale3D` (`self.Mesh_04`) (`KismetMathLibrary.VLerp` (`self.Original Scale 4`) (`self.Mesh_4_Scale`) (`self.Alpha`)))
                    (`SceneComponent.K2_SetRelativeRotation` (`self.Mesh_05`) (`KismetMathLibrary.RLerp` (`self.OriginalRotation_5`) (`self.Mesh_5_Rotation`) (`self.Alpha`)) false false)
                    (`SceneComponent.K2_SetRelativeLocation` (`self.Mesh_05`) (`KismetMathLibrary.VLerp` (`self.OriginalLocation_5`) (`self.Mesh_5_Location`) (`self.Alpha`)) false false)
                    (`SceneComponent.SetRelativeScale3D` (`self.Mesh_05`) (`KismetMathLibrary.VLerp` (`self.Original Scale 5`) (`self.Mesh_5_Scale`) (`self.Alpha`)))
                    (`SceneComponent.K2_SetRelativeRotation` (`self.Mesh_06`) (`KismetMathLibrary.RLerp` (`self.OriginalRotation_6`) (`self.Mesh_6_Rotation`) (`self.Alpha`)) false false)
                    (`SceneComponent.K2_SetRelativeLocation` (`self.Mesh_06`) (`KismetMathLibrary.VLerp` (`self.OriginalLocation_6`) (`self.Mesh_6_Location`) (`self.Alpha`)) false false)
                    (`SceneComponent.SetRelativeScale3D` (`self.Mesh_06`) (`KismetMathLibrary.VLerp` (`self.Original Scale 6`) (`self.Mesh_6_Scale`) (`self.Alpha`)))
                    (`SceneComponent.K2_SetRelativeRotation` (`self.Mesh_07`) (`KismetMathLibrary.RLerp` (`self.OriginalRotation_7`) (`self.Mesh_7_Rotation`) (`self.Alpha`)) false false)
                    (`SceneComponent.K2_SetRelativeLocation` (`self.Mesh_07`) (`KismetMathLibrary.VLerp` (`self.OriginalLocation_7`) (`self.Mesh_7_Location`) (`self.Alpha`)) false false)
                    (`SceneComponent.SetRelativeScale3D` (`self.Mesh_07`) (`KismetMathLibrary.VLerp` (`self.Original Scale 7`) (`self.Mesh_7_Scale`) (`self.Alpha`))))))
              (:`then_1`
                ;;[0 0 0] Sound
                (`KismetSystemLibrary.Delay` (`self.Delay Before Forward Sound`))
                (`GameplayStatics.PlaySound2D` (`self.Forward Sound`) 1.0 1.0 0.0 null null)))
            (else
              (set `self.TriggerInteraction?` true)
              (`|ExecutionSequence`
                (:`then_0`
                  (goto _label :!via `Reverse`))
                (:`then_1`
                  (`KismetSystemLibrary.Delay` (`self.Delay Before Backward Sound`))
                  (`GameplayStatics.PlaySound2D` (`self.Backward Sound`) 1.0 1.0 0.0 null null))))))
        (:`then_1`
          (bind (_direction_2 _alpha_2) (`Timeline|Timeline` :!label _label_2)
            (:`Update`
              (set `self.Alpha` _alpha_2))))
        (:`then_2`
          (`KismetSystemLibrary.Delay` 0.5)
          (goto _label_2 :!via `Reverse`))))))

(event `/Game/InfinityAssets/BP/Sculpture/BPI_InfinityTrigger.Lift UP Anim`
  ;[0 0 0] Up lift Gravity
  (if (`self.GravityEnable?`)
    (set `self.GravityEnable?` false)
    (bind (_direction _newtrack_0) (`Timeline|Lift UP` :!via `Reverse` :!label _label_3)
      (:`Update`
        (bind _returnvalue (`KismetMathLibrary.Lerp` 0.0 (`KismetMathLibrary.FClamp` 0.0 5.0 15.0) _newtrack_0))
        (`SceneComponent.K2_SetRelativeLocationAndRotation` (`self.DefaultSceneRoot`) (`KismetMathLibrary.MakeVector` 0.0 0.0 (`KismetMathLibrary.Lerp` 0.0 (`KismetMathLibrary.FClamp` 0.0 60.0 85.0) _newtrack_0)) (`KismetMathLibrary.MakeRotator` _returnvalue _returnvalue) false false)))
    (else
      (set `self.GravityEnable?` true)
      (goto _label_3))))

(event `/Game/InfinityAssets/BP/Sculpture/BPI_InfinityTrigger.Hide Decore and other`
  (bind _sm_decor_2 (`self.SM_Decor_2`))
  ;[0 0 0] Hide Decor
  (`/Engine/EditorBlueprintResources/StandardMacros.FlipFlop`
    (:`A`
      (`SceneComponent.SetVisibility` _sm_decor_2 true false)
      (`SceneComponent.SetVisibility` (`self.SM_Decor_4`) true false)
      (`SceneComponent.SetVisibility` (`self.SM_Decor_5`) true false)
      (`SceneComponent.SetVisibility` (`self.SM_Decor_6`) true false)
      (`SceneComponent.SetVisibility` (`self.SM_Decor_3`) true false)
      (`SceneComponent.SetVisibility` (`self.SM_Decor_7`) true false)
      (`SceneComponent.SetVisibility` (`self.SM_Decor_8`) true false)
      (`SceneComponent.SetVisibility` (`self.SM_Decor_1`) true false)
      (set `self.Decor Visiblity` false))
    (:`B`
      (`SceneComponent.SetVisibility` _sm_decor_2 false false)
      (`SceneComponent.SetVisibility` (`self.SM_Decor_4`) false false)
      (`SceneComponent.SetVisibility` (`self.SM_Decor_5`) false false)
      (`SceneComponent.SetVisibility` (`self.SM_Decor_6`) false false)
      (`SceneComponent.SetVisibility` (`self.SM_Decor_3`) false false)
      (`SceneComponent.SetVisibility` (`self.SM_Decor_7`) false false)
      (`SceneComponent.SetVisibility` (`self.SM_Decor_1`) false false)
      (`SceneComponent.SetVisibility` (`self.SM_Decor_8`) false false)
      (set `self.Decor Visiblity` true))))

(fn `ApplySavedEmissiveState`
  (params (TurnOn :type Boolean))
  (for (_array_element _array_index) (`self.EmissiveMIDs`)
    (if TurnOn
      (`MaterialInstanceDynamic.SetScalarParameterValue` _array_element "EmissiveStrength" (`|GetArrayItem` (`self.EmissiveDefaultStrengths`) _array_index))
      (else
        (`MaterialInstanceDynamic.SetScalarParameterValue` _array_element "EmissiveStrength" 0.0)))))

(fn `OriginalLocation`
  (bind _mesh_01 (`self.Mesh_01`))
  (bind _mesh_02 (`self.Mesh_02`))
  (bind _mesh_06 (`self.Mesh_06`))
  (bind _mesh_05 (`self.Mesh_05`))
  (bind _mesh_03 (`self.Mesh_03`))
  (bind _mesh_04 (`self.Mesh_04`))
  (bind _mesh_07 (`self.Mesh_07`))
  ;[0 0 0] Original Location
  (set `self.OriginalLocation_1` (`SceneComponent.RelativeLocation` _mesh_01))
  (set `self.OriginalRotation_1` (`SceneComponent.RelativeRotation` _mesh_01))
  (set `self.Original Scale 1` (`SceneComponent.RelativeScale3D` _mesh_01))
  (set `self.OriginalLocation_2` (`SceneComponent.RelativeLocation` _mesh_02))
  (set `self.OriginalRotation_2` (`SceneComponent.RelativeRotation` _mesh_02))
  (set `self.Original Scale 2` (`SceneComponent.RelativeScale3D` _mesh_02))
  (set `self.OriginalLocation_4` (`SceneComponent.RelativeLocation` _mesh_04))
  (set `self.OriginalRotation_4` (`SceneComponent.RelativeRotation` _mesh_04))
  (set `self.Original Scale 4` (`SceneComponent.RelativeScale3D` _mesh_04))
  (set `self.OriginalLocation_7` (`SceneComponent.RelativeLocation` _mesh_07))
  (set `self.OriginalRotation_7` (`SceneComponent.RelativeRotation` _mesh_07))
  (set `self.Original Scale 7` (`SceneComponent.RelativeScale3D` _mesh_07))
  (set `self.OriginalLocation_6` (`SceneComponent.RelativeLocation` _mesh_06))
  (set `self.OriginalRotation_6` (`SceneComponent.RelativeRotation` _mesh_06))
  (set `self.Original Scale 6` (`SceneComponent.RelativeScale3D` _mesh_06))
  (set `self.OriginalLocation_5` (`SceneComponent.RelativeLocation` _mesh_05))
  (set `self.OriginalRotation_5` (`SceneComponent.RelativeRotation` _mesh_05))
  (set `self.Original Scale 5` (`SceneComponent.RelativeScale3D` _mesh_05))
  (set `self.OriginalLocation_3` (`SceneComponent.RelativeLocation` _mesh_03))
  (set `self.OriginalRotation_3` (`SceneComponent.RelativeRotation` _mesh_03))
  (set `self.Original Scale 3` (`SceneComponent.RelativeScale3D` _mesh_03)))

(fn `SwitchMaterialOnMesh`
  (params (MeshIndex :type Integer) (NewMaterial :type "MaterialInstance Object Reference"))
  (bind _output (`|GetArrayItem` (`self.MeshComponentsArray`) MeshIndex))
  (`/Engine/EditorBlueprintResources/StandardMacros.IsValid` _output
    (:`Is Valid`
      (`PrimitiveComponent.SetMaterial` _output 0 NewMaterial))))

(fn `SyncMeshesToVariables`
  (bind _mesh_01 (`self.Mesh_01`))
  (bind _mesh_02 (`self.Mesh_02`))
  (bind _mesh_06 (`self.Mesh_06`))
  (bind _mesh_03 (`self.Mesh_03`))
  (bind _mesh_01_2 (`self.Mesh_01`))
  (bind _mesh_05 (`self.Mesh_05`))
  (bind _mesh_03_2 (`self.Mesh_03`))
  (bind _mesh_04 (`self.Mesh_04`))
  (bind _mesh_07 (`self.Mesh_07`))
  (bind _mesh_05_2 (`self.Mesh_05`))
  (bind _mesh_06_2 (`self.Mesh_06`))
  (bind _mesh_07_2 (`self.Mesh_07`))
  (bind _mesh_02_2 (`self.Mesh_02`))
  (bind _mesh_04_2 (`self.Mesh_04`))
  (if (`self.sy_OriinalEnabled`)
    ;[0 0 0] Original
    (set `self.OriginalLocation_1` (`SceneComponent.RelativeLocation` _mesh_01))
    (set `self.OriginalRotation_1` (`SceneComponent.RelativeRotation` _mesh_01))
    (set `self.Original Scale 1` (`SceneComponent.RelativeScale3D` _mesh_01))
    (set `self.OriginalLocation_2` (`SceneComponent.RelativeLocation` _mesh_02))
    (set `self.OriginalRotation_2` (`SceneComponent.RelativeRotation` _mesh_02))
    (set `self.Original Scale 2` (`SceneComponent.RelativeScale3D` _mesh_02))
    (set `self.OriginalLocation_4` (`SceneComponent.RelativeLocation` _mesh_04))
    (set `self.OriginalRotation_4` (`SceneComponent.RelativeRotation` _mesh_04))
    (set `self.Original Scale 4` (`SceneComponent.RelativeScale3D` _mesh_04))
    (set `self.OriginalLocation_7` (`SceneComponent.RelativeLocation` _mesh_07))
    (set `self.OriginalRotation_7` (`SceneComponent.RelativeRotation` _mesh_07))
    (set `self.Original Scale 7` (`SceneComponent.RelativeScale3D` _mesh_07))
    (set `self.OriginalLocation_6` (`SceneComponent.RelativeLocation` _mesh_06))
    (set `self.OriginalRotation_6` (`SceneComponent.RelativeRotation` _mesh_06))
    (set `self.Original Scale 6` (`SceneComponent.RelativeScale3D` _mesh_06))
    (set `self.OriginalLocation_5` (`SceneComponent.RelativeLocation` _mesh_05))
    (set `self.OriginalRotation_5` (`SceneComponent.RelativeRotation` _mesh_05))
    (set `self.Original Scale 5` (`SceneComponent.RelativeScale3D` _mesh_05))
    (set `self.OriginalLocation_3` (`SceneComponent.RelativeLocation` _mesh_03_2))
    (set `self.OriginalRotation_3` (`SceneComponent.RelativeRotation` _mesh_03_2))
    (set `self.Original Scale 3` (`SceneComponent.RelativeScale3D` _mesh_03_2))
    (else
      ;[0 0 0] New
      (`|ExecutionSequence`
        (:`then_0`
          (set `self.Mesh_5_Location` (`SceneComponent.RelativeLocation` _mesh_05_2))
          (set `self.Mesh_5_Rotation` (`SceneComponent.RelativeRotation` _mesh_05_2))
          (set `self.Mesh_5_Scale` (`SceneComponent.RelativeScale3D` _mesh_05_2)))
        (:`then_1`
          (set `self.Mesh_6_Location` (`SceneComponent.RelativeLocation` _mesh_06_2))
          (set `self.Mesh_6_Rotation` (`SceneComponent.RelativeRotation` _mesh_06_2))
          (set `self.Mesh_6_Scale` (`SceneComponent.RelativeScale3D` _mesh_06_2)))
        (:`then_2`
          (set `self.Mesh_7_Location` (`SceneComponent.RelativeLocation` _mesh_07_2))
          (set `self.Mesh_7_Rotation` (`SceneComponent.RelativeRotation` _mesh_07_2))
          (set `self.Mesh_7_Scale` (`SceneComponent.RelativeScale3D` _mesh_07_2)))
        (:`then_3`
          (set `self.Mesh_3_Location` (`SceneComponent.RelativeLocation` _mesh_03))
          (set `self.Mesh_3_Rotation` (`SceneComponent.RelativeRotation` _mesh_03))
          (set `self.Mesh_3_Scale` (`SceneComponent.RelativeScale3D` _mesh_03)))
        (:`then_4`
          (set `self.Mesh_1_Location` (`SceneComponent.RelativeLocation` _mesh_01_2))
          (set `self.Mesh_1_Rotation` (`SceneComponent.RelativeRotation` _mesh_01_2))
          (set `self.Mesh_1_Scale` (`SceneComponent.RelativeScale3D` _mesh_01_2)))
        (:`then_5`
          (set `self.Mesh_2_Location` (`SceneComponent.RelativeLocation` _mesh_02_2))
          (set `self.Mesh_2_Rotation` (`SceneComponent.RelativeRotation` _mesh_02_2))
          (set `self.Mesh_2_Scale` (`SceneComponent.RelativeScale3D` _mesh_02_2)))
        (:`then_6`
          (set `self.Mesh_4_Location` (`SceneComponent.RelativeLocation` _mesh_04_2))
          (set `self.Mesh_4_Rotation` (`SceneComponent.RelativeRotation` _mesh_04_2))
          (set `self.Mesh_4_Scale` (`SceneComponent.RelativeScale3D` _mesh_04_2)))))))

(fn `ToggleEmissiveMaterials`
  (params (TurnOn :type Boolean))
  (for (_array_element _array_index) (`self.EmissiveMeshComponents`)
    (if TurnOn
      (bind _output (`|GetArrayItem` (`self.EmissiveMaterialIndices`) _array_index))
      (`PrimitiveComponent.SetMaterial` _array_element _output (`|GetArrayItem` (`self.OriginalEmissiveMaterials`) _array_index))
      (else
        (`PrimitiveComponent.SetMaterial` _array_element _output (`self.OffMaterial`))))))

(fn `UserConstructionScript`
  (`|ExecutionSequence`
    (:`then_1`
      ;[0 0 0] Dcor Visiblity
      (`SceneComponent.SetVisibility` (`self.SM_Decor_2`) (`self.Decor Visiblity`) false)
      (`SceneComponent.SetVisibility` (`self.SM_Decor_4`) (`self.Decor Visiblity`) false)
      (`SceneComponent.SetVisibility` (`self.SM_Decor_5`) (`self.Decor Visiblity`) false)
      (`SceneComponent.SetVisibility` (`self.SM_Decor_6`) (`self.Decor Visiblity`) false)
      (`SceneComponent.SetVisibility` (`self.SM_Decor_3`) (`self.Decor Visiblity`) false)
      (`SceneComponent.SetVisibility` (`self.SM_Decor_7`) (`self.Decor Visiblity`) false)
      (`SceneComponent.SetVisibility` (`self.SM_Decor_8`) (`self.Decor Visiblity`) false)
      (`SceneComponent.SetVisibility` (`self.SM_Decor_1`) (`self.Decor Visiblity`) false))))