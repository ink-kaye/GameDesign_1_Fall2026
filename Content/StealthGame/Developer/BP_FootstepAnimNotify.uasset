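; Animation notify that plays a running footstep sound matched to the surface beneath the animated mesh's owner.
; Each notify traces 200 units along the owner's downward axis on the Visibility channel and switches on the hit's physical surface type.
; Grass, wood and concrete each play their own fixed sound, positioned at the world origin rather than at the character or hit point.
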(fn `Received_Notify`
  (params (MeshComp :type "SkeletalMeshComponent Object Reference") (Animation :type "AnimSequenceBase Object Reference") (EventReference :type "AnimNotifyEventReference Structure (by ref)"))
  (returns (ReturnValue :type Boolean))
  (bind _returnvalue (`ActorComponent.GetOwner` MeshComp))
  (bind _returnvalue_2 (`Actor.K2_GetActorLocation` _returnvalue))
  (bind _outhit (`KismetSystemLibrary.LineTraceSingle` _returnvalue_2 (+ _returnvalue_2 (* (`Actor.GetActorUpVector` _returnvalue) -200.0)) "TraceTypeQuery1"))
  (if true
    (switch `EPhysicalSurface` (`GameplayStatics.GetSurfaceType` _outhit)
      (:`SurfaceType1`
        (`GameplayStatics.PlaySoundAtLocation` "/Game/StealthGame/Effects/SFX/Footsteps/A_Dirt_Run_002.A_Dirt_Run_002" (0.0 0.0 0.0) (struct) 1.0 1.0 0.0 null null null null))
      (:`SurfaceType2`
        (`GameplayStatics.PlaySoundAtLocation` "/Game/StealthGame/Effects/SFX/Footsteps/A_Wood_Run_002.A_Wood_Run_002" (0.0 0.0 0.0) (struct) 1.0 1.0 0.0 null null null null))
      (:`SurfaceType3`
        (`GameplayStatics.PlaySoundAtLocation` "/Game/StealthGame/Effects/SFX/Footsteps/A_Concrete_Run_001.A_Concrete_Run_001" (0.0 0.0 0.0) (struct) 1.0 1.0 0.0 null null null null)))
    (return false)))