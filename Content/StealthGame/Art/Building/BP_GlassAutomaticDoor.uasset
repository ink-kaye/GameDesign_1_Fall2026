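; BP_GlassAutomaticDoor is an automatic sliding glass double door that opens when something overlaps its Box trigger.
; Overlap begin plays the SlideOpenDoor timeline, whose DoorSlide value lerps DoorLeft and DoorRight apart along local Y.
; Overlap end reverses the timeline to close it, with no filtering of the overlapping actor.
; BeginPlay caches the GI_Instance game instance, which the door logic does not use.
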(event `self.ReceiveBeginPlay`
  (bind _asgi_instance (cast `/Game/StealthGame/Core/Interactables/GI_Instance` (`GameplayStatics.GetGameInstance`)))
  (set `self.As GI Instance` _asgi_instance))

(event `self.Box.OnComponentBeginOverlap`
  (params (OverlappedComponent :type "PrimitiveComponent Object Reference") (OtherActor :type "Actor Object Reference") (OtherComp :type "PrimitiveComponent Object Reference") (OtherBodyIndex :type Integer) (bFromSweep :type Boolean) (SweepResult :type "HitResult Structure (by ref)"))
  (bind (_direction _doorslide) (`Timeline|SlideOpenDoor` :!label _label)
    (:`Update`
      (`SceneComponent.K2_SetRelativeLocation` (`self.DoorRight`) (`KismetMathLibrary.MakeVector` 0.0 (`KismetMathLibrary.Lerp` -108.0 -324.0 _doorslide) 155.0) false false)
      (`SceneComponent.K2_SetRelativeLocation` (`self.DoorLeft`) (`KismetMathLibrary.MakeVector` 0.0 (`KismetMathLibrary.Lerp` 120.0 350.0 _doorslide) 155.0) false false))))

(event `self.Box.OnComponentEndOverlap`
  (params (OverlappedComponent :type "PrimitiveComponent Object Reference") (OtherActor :type "Actor Object Reference") (OtherComp :type "PrimitiveComponent Object Reference") (OtherBodyIndex :type Integer))
  (goto _label :!via `Reverse`))

(fn `UserConstructionScript`)