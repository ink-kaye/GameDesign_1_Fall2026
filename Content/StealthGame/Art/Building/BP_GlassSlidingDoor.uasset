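; BP_GlassSlidingDoor is an interactable double door that, despite its name, swings rather than slides.
; Interact drives two FlipFlops that alternately play a timeline from start or reverse it.
; The timelines lerp the yaw of Pivot and Pivot1 toward 90 degrees in opposite directions.
; BeginPlay caches the GI_Instance game instance, which the door logic does not use.
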(event `self.ReceiveBeginPlay`
  (bind _asgi_instance (cast `/Game/StealthGame/Core/Interactables/GI_Instance` (`GameplayStatics.GetGameInstance`)))
  (set `self.As GI Instance` _asgi_instance))

(event `/Game/StealthGame/Core/Interactables/BPI_Interact.Interact`
  (`|ExecutionSequence`
    (:`then_0`
      (`/Engine/EditorBlueprintResources/StandardMacros.FlipFlop`
        (:`A`
          (bind (_direction _opendoor) (`Timeline|Timeline` :!via `PlayFromStart` :!label _label)
            (:`Update`
              (`SceneComponent.K2_SetRelativeRotation` (`self.Pivot`) (`KismetMathLibrary.MakeRotator` 0.0 0.0 (`KismetMathLibrary.Lerp` 0.0 90.0 _opendoor)) false false))))
        (:`B`
          (goto _label :!via `Reverse`))))
    (:`then_1`
      (`/Engine/EditorBlueprintResources/StandardMacros.FlipFlop`
        (:`A`
          (bind (_direction_2 _opendoor_2) (`Timeline|Timeline_0` :!via `PlayFromStart` :!label _label_2)
            (:`Update`
              (`SceneComponent.K2_SetRelativeRotation` (`self.Pivot1`) (`KismetMathLibrary.MakeRotator` 0.0 0.0 (`KismetMathLibrary.Lerp` 0.0 -90.0 _opendoor_2)) false false))))
        (:`B`
          (goto _label_2 :!via `Reverse`))))))

(fn `UserConstructionScript`)