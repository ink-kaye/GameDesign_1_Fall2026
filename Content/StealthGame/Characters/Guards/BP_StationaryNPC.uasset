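; Stationary NPC that the player can talk to, showing its lines in an on-screen dialogue widget.
; Each Talk event, triggered from outside this graph, advances through the Dialogue array, creating WBP_Dialogue when needed and removing it after the last line to reset the conversation.
; TargetZone overlaps add and remove a WBP_NpcInteract prompt for the custom third-person character; the trailing Delay after showing it drives nothing.
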(event `/Game/StealthGame/Characters/Guards/BPI_Dialogue.Talk`
  (`/Engine/EditorBlueprintResources/StandardMacros.IncrementInt` (`self.TalkIndex`)
    (:`  `
      (if (< (`self.TalkIndex`) (`KismetArrayLibrary.Array_Length` (`self.Dialogue`)))
        (`self.UI`
          (:`then`
            _)
          (:`else`
            (bind _returnvalue (`|CreateWidget` "/Game/StealthGame/Characters/Guards/WBP_Dialogue.WBP_Dialogue_C" (`GameplayStatics.GetPlayerController` 0)))
            (bind _output_get (set `self.UI` _returnvalue))
            (`UserWidget.AddToViewport` _output_get 0)))
        (`TextBlock.SetText` (`/Game/StealthGame/Characters/Guards/WBP_Dialogue.EasedroppingDialogue` (`self.UI`)) (`KismetTextLibrary.Conv_StringToText` (`|GetArrayItem` (`self.Dialogue`) (`self.TalkIndex`))))
        (else
          (`Widget.RemoveFromParent` (`self.UI`))
          (set `self.TalkIndex` -1)
          (set `self.UI` null))))))

(event `self.TargetZone.OnComponentBeginOverlap`
  (params (OverlappedComponent :type "PrimitiveComponent Object Reference") (OtherActor :type "Actor Object Reference") (OtherComp :type "PrimitiveComponent Object Reference") (OtherBodyIndex :type Integer) (bFromSweep :type Boolean) (SweepResult :type "HitResult Structure (by ref)"))
  (cast `/Game/StealthGame/Core/Characters/PlayerCharacter/BP_ThirdPersonCharacterCustom` OtherActor)
  (bind _returnvalue (`|CreateWidget` "/Game/StealthGame/Characters/Guards/WBP_NpcInteract.WBP_NpcInteract_C"))
  (`UserWidget.AddToViewport` _returnvalue 0)
  (`KismetSystemLibrary.Delay` 7.0))

(event `self.TargetZone.OnComponentEndOverlap`
  (params (OverlappedComponent :type "PrimitiveComponent Object Reference") (OtherActor :type "Actor Object Reference") (OtherComp :type "PrimitiveComponent Object Reference") (OtherBodyIndex :type Integer))
  (cast `/Game/StealthGame/Core/Characters/PlayerCharacter/BP_ThirdPersonCharacterCustom` OtherActor)
  (`Widget.RemoveFromParent` (stale `self.TargetZone.OnComponentBeginOverlap` _returnvalue)))

(fn `UserConstructionScript`)