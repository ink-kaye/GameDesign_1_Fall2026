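; BP_KeyCardT3 is an interactable tier 3 keycard pickup for the stealth game.
; BeginPlay caches the player as BP_ThirdPersonCharacterCustom.
; The first Interact calls T3KeycardGrabbed on that character and shows a WBP_KeyNotif widget with the key's name.
; It then calls SetActorHiddenInGame with false, which leaves the card visible, and destroys the actor after a short delay.
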(event `self.ReceiveBeginPlay`
  (bind _asbp_third_person_character_custom (cast `/Game/StealthGame/Core/Characters/PlayerCharacter/BP_ThirdPersonCharacterCustom` (`GameplayStatics.GetPlayerCharacter` 0)))
  (set `self.PlayerRef` _asbp_third_person_character_custom))

(event `self.Interact`
  (`/Engine/EditorBlueprintResources/StandardMacros.DoOnce` false
    (:`Completed`
      (`/Game/StealthGame/Core/Characters/PlayerCharacter/BP_ThirdPersonCharacterCustom.T3 Keycard grabbed` (`self.PlayerRef`))
      (bind _returnvalue (`|CreateWidget` "/Game/StealthGame/Core/Interactables/KeyCards/WBP_KeyNotif.WBP_KeyNotif_C"))
      (`TextBlock.SetText` (`/Game/StealthGame/Core/Interactables/KeyCards/WBP_KeyNotif.KeyName` _returnvalue) (`self.KeyName`))
      (`UserWidget.AddToViewport` _returnvalue 0)
      (`self.SetActorHiddenInGame` false)
      (`KismetSystemLibrary.Delay` 0.2)
      (`self.K2_DestroyActor`))))

(fn `UserConstructionScript`)