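; Master-tier card reader interactable that opens up access through its linked door and laser door when the player holds the Master keycard.
; BeginPlay caches GI_Instance, and Interact checks its HasKeycardMaster flag.
; With the card, it messages the laser door on each use, then once messages the door and shows a success widget.
; Without it, a notification widget displays the reader's tier text.
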(event `self.ReceiveBeginPlay`
  (bind _asgi_instance (cast `/Game/StealthGame/Core/Interactables/GI_Instance` (`GameplayStatics.GetGameInstance`)))
  (set `self.GameIntanceRef` _asgi_instance))

(event `/Game/StealthGame/Core/Interactables/BPI_Interact.Interact`
  (if (`/Game/StealthGame/Core/Interactables/GI_Instance.bHasKeycardMaster` (`self.GameIntanceRef`))
    (message `/Game/StealthGame/Core/Interactables/BPI_Door.Has Key` (`self.LaserDoorRef`))
    (if true
      (`/Engine/EditorBlueprintResources/StandardMacros.DoOnce` false
        (:`Completed`
          (message `/Game/StealthGame/Core/Interactables/BPI_Door.Has Key` (`self.DoorRef`))
          (bind _returnvalue (`|CreateWidget` "/Game/StealthGame/Core/Interactables/WBP_KeyCardSuccess.WBP_KeyCardSuccess_C"))
          (`UserWidget.AddToViewport` _returnvalue 0))))
    (else
      (bind _returnvalue_2 (`|CreateWidget` "/Game/StealthGame/Core/Interactables/KeyCards/WBP_CardReaderNotif.WBP_CardReaderNotif_C"))
      (`TextBlock.SetText` (`/Game/StealthGame/Core/Interactables/KeyCards/WBP_CardReaderNotif.CardReaderTier` _returnvalue_2) (`self.Card Reader Text`))
      (`UserWidget.AddToViewport` _returnvalue_2 0)
      (`KismetSystemLibrary.Delay` 0.2))))

(fn `UserConstructionScript`)