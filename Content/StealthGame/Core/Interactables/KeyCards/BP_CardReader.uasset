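; BP_CardReader is an interactable keycard reader that notifies a linked door when the player holds a keycard.
; On Interact it checks keycard flags on the game instance, cached at BeginPlay, and accepts any tier, including master.
; Success fires once, calling HasKeyMessage on DoorRef and showing a success widget.
; Without a card, it shows a notification widget labeled with the reader's tier text.
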(event `self.ReceiveBeginPlay`
  (bind _asgi_instance (cast `/Game/StealthGame/Core/Interactables/GI_Instance` (`GameplayStatics.GetGameInstance`)))
  (set `self.As GI Instance` _asgi_instance))

(event `/Game/StealthGame/Core/Interactables/BPI_Interact.Interact`
  (bind _as_gi_instance (`self.As GI Instance`))
  (if (or (`/Game/StealthGame/Core/Interactables/GI_Instance.bHasKeycard` _as_gi_instance) (`/Game/StealthGame/Core/Interactables/GI_Instance.bHasKeycardT2` _as_gi_instance) (`/Game/StealthGame/Core/Interactables/GI_Instance.bHasKeycardT3` _as_gi_instance) (`/Game/StealthGame/Core/Interactables/GI_Instance.bHasKeycardMaster` _as_gi_instance))
    (`/Engine/EditorBlueprintResources/StandardMacros.DoOnce` false
      (:`Completed`
        (message `/Game/StealthGame/Core/Interactables/BPI_Door.Has Key` (`self.DoorRef`))
        (bind _returnvalue (`|CreateWidget` "/Game/StealthGame/Core/Interactables/WBP_KeyCardSuccess.WBP_KeyCardSuccess_C"))
        (`UserWidget.AddToViewport` _returnvalue 0)))
    (else
      (bind _returnvalue_2 (`|CreateWidget` "/Game/StealthGame/Core/Interactables/KeyCards/WBP_CardReaderNotif.WBP_CardReaderNotif_C"))
      (`TextBlock.SetText` (`/Game/StealthGame/Core/Interactables/KeyCards/WBP_CardReaderNotif.CardReaderTier` _returnvalue_2) (`self.CardReadertext`))
      (`UserWidget.AddToViewport` _returnvalue_2 0)
      (`self.SetActorHiddenInGame` false)
      (`KismetSystemLibrary.Delay` 0.2))))

(fn `UserConstructionScript`)