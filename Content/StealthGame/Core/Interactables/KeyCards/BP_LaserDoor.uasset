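; BP_LaserDoor is a laser barrier in the stealth game that drops temporarily when its HasKey event receives a key card swipe.
; A successful swipe adds the WBP_LasersDown widget to the viewport, hides the actor and disables its collision, then restores both after a ten-second Delay.
; CanBeSwiped blocks repeat swipes during that window, though the rejection message says seven seconds.
; BeginPlay caches the GI_Instance, which is otherwise unused here.
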(event `self.ReceiveBeginPlay`
  (bind _asgi_instance (cast `/Game/StealthGame/Core/Interactables/GI_Instance` (`GameplayStatics.GetGameInstance`)))
  (set `self.As GI Instance` _asgi_instance))

(event `/Game/StealthGame/Core/Interactables/BPI_Door.Has Key`
  (if (`self.bCanBeSwiped`)
    (`KismetSystemLibrary.PrintString` "Swipe received")
    (set `self.bCanBeSwiped` false)
    (bind _returnvalue (`|CreateWidget` "/Game/StealthGame/Core/Interactables/KeyCards/WBP_LasersDown.WBP_LasersDown_C"))
    (`UserWidget.AddToViewport` _returnvalue 0)
    (`self.SetActorHiddenInGame` true)
    (`self.SetActorEnableCollision` false)
    (`KismetSystemLibrary.Delay` 10.0)
    (`self.SetActorHiddenInGame` false)
    (`self.SetActorEnableCollision` true)
    (set `self.bCanBeSwiped` true)
    (else
      (`KismetSystemLibrary.PrintString` "Swipe again in 7 seconds"))))

(fn `UserConstructionScript`)