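; BP_MuseumDoor is an interactable museum door that stays locked until its HasKey event unlocks it.
; When unlocked, Interact alternates through a FlipFlop between playing and reversing a timeline that swings the door mesh's yaw open and closed.
; When locked, Interact shows a WBP_DoorLockedMessage widget labelled with the door's type.
; BeginPlay caches the GI_Instance game instance, which the rest of the graph does not use.
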(event `self.ReceiveBeginPlay`
  (bind _asgi_instance (cast `/Game/StealthGame/Core/Interactables/GI_Instance` (`GameplayStatics.GetGameInstance`)))
  (set `self.As GI Instance_0` _asgi_instance))

(event `/Game/StealthGame/Core/Interactables/BPI_Interact.Interact`
  (if (`self.bDoorUnlocked`)
    (`/Engine/EditorBlueprintResources/StandardMacros.FlipFlop`
      (:`A`
        (bind (_direction _opendoor) (`Timeline|open a door` :!via `PlayFromStart` :!label _label)
          (:`Update`
            (`SceneComponent.K2_SetRelativeRotation` (`self.SM_ConvStore_Building_Door_03`) (`KismetMathLibrary.MakeRotator` 0.0 0.0 (`KismetMathLibrary.Lerp` 0.0 90.0 _opendoor)) false false))))
      (:`B`
        (goto _label :!via `Reverse`)))
    (else
      (bind _returnvalue (`|CreateWidget` "/Game/StealthGame/Core/Interactables/WBP_DoorLockedMessage.WBP_DoorLockedMessage_C"))
      (`TextBlock.SetText` (`/Game/StealthGame/Core/Interactables/WBP_DoorLockedMessage.TypeOfDoor` _returnvalue) (`self.TypeOfDoor`))
      (`UserWidget.AddToViewport` _returnvalue 0)
      (`self.SetActorHiddenInGame` false)
      (`KismetSystemLibrary.Delay` 0.2))))

(event `/Game/StealthGame/Core/Interactables/BPI_Door.Has Key`
  (set `self.bDoorUnlocked` true))

(fn `UserConstructionScript`)